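; Target actor that takes hits, awards score to whoever hit it, and is destroyed when its health runs out.
; On BeginPlay it creates a dynamic material for its cylinder and registers itself with the GameMode.
; Each hit sends score to the hitter, subtracts damage and lerps the material color from green toward red by remaining health.
; At zero health it sends bonus score, unregisters from the GameMode and destroys itself.
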(event EventHandleWasHit
  (params (Hitter :type Actor%20Object%20Reference) (DamageValue :type Integer))
  (Variables|Default|SetHitter Hitter)
  (Variables|Default|SetDamageValue DamageValue)
  (Class|FPS-Controller-BPI|HandleUpdateScore(Message) (Variables|Default|GetHitter) (Variables|Default|GetTargetScoreValue))
  (Variables|Default|SetTargetHealthValue (- (Variables|Default|GetTargetHealthValue) (Variables|Default|GetDamageValue)))
  (CallFunction|SetColor)
  (if (<= (Variables|Default|GetTargetHealthValue) 0)
    (Class|FPS-Controller-BPI|HandleUpdateScore(Message) (Variables|Default|GetHitter) (Variables|Default|GetBonusValue))
    (Class|FPS-Gamemode-BPI|RemoveTarget(Message) (Game|GetGameMode))
    (Actor|DestroyActor)))

(event EventBeginPlay
  (Variables|Default|SetStartingHealthValue (Variables|Default|GetTargetHealthValue))
  (bind _returnvalue (Rendering|Material|CreateDynamicMaterialInstance "/Game/Materials/TargetMat.TargetMat" :!class /Script/Engine.KismetMaterialLibrary))
  (Variables|Default|SetDynamicMat _returnvalue)
  (Rendering|Material|SetMaterial (Variables|Default|GetCylinder) 0 (Variables|Default|GetDynamicMat))
  (CallFunction|SetColor)
  (Class|FPS-Gamemode-BPI|AddTarget(Message) (Game|GetGameMode)))

(fn ConstructionScript)

(fn SetColor
  (Rendering|Material|SetVectorParameterValue (Variables|Default|GetDynamicMat) "Color" (Math|Color|Lerp(LinearColor) "(R=1.000000,G=0.000000,B=0.000000,A=1.000000)" "(R=0.000000,G=0.500000,B=0.000000,A=1.000000)" (/ (Math|Conversions|ToFloat(Integer) (Variables|Default|GetTargetHealthValue)) (Math|Conversions|ToFloat(Integer) (Variables|Default|GetStartingHealthValue)))) :!class /Script/Engine.MaterialInstanceDynamic)
  (return))