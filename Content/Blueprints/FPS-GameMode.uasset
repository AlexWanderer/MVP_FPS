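; FPS game mode that tracks the number of remaining targets and ends the game when none are left.
; AddTarget and RemoveTarget events adjust the counter, and removal calls HandleGameOver once it reaches zero or below.
; HandleGameOver shows a GameOverScreen widget and switches player 0 to UI-only input, keeping the mouse cursor hidden.
; HandleGameStart sets game-only input and hides the cursor.
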(event EventAddTarget
  (Variables|Default|SetTargetsRemaining (+ (Variables|Default|GetTargetsRemaining) 1)))

(event EventRemoveTarget
  (Variables|Default|SetTargetsRemaining (- (Variables|Default|GetTargetsRemaining) 1))
  (if (<= (Variables|Default|GetTargetsRemaining) 0)
    (CallFunction|HandleGameOver)))

(event EventHandleGameStart
  (bind _returnvalue (Game|GetPlayerController 0))
  (Input|SetInputModeGameOnly _returnvalue)
  (Variables|/Script/Engine.PlayerController|SetbShowMouseCursor _returnvalue false))

(fn ConstructionScript)

(fn HandleGameOver
  (bind _returnvalue (Game|GetPlayerController 0))
  (bind _returnvalue_2 (UserInterface|CreateWidget "/Game/Blueprints/UI/GameOverScreen.GameOverScreen_C"))
  (UserInterface|Viewport|AddtoViewport _returnvalue_2 0)
  (Input|SetInputModeUIOnly _returnvalue 0 false)
  (Variables|/Script/Engine.PlayerController|SetbShowMouseCursor _returnvalue false))